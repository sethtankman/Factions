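; Clickable board square actor that signals its selection and shows hover, enemy-occupied and moveable states through material swaps on its static mesh.
; Hover caches the current material and restores it when the cursor leaves; releasing a click calls the SetSelectedSquare dispatcher with itself.
; A SetEnemyOccupied dispatcher binding updates occupancy and refreshes the material.
; SetMoveable picks a material from movability and occupancy, while SetVisibility toggles the mesh.
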(event OnReleased(StaticMesh)
  (params (TouchedComponent :type Primitive%20Component%20Object%20Reference) (ButtonReleased :type Key%20Structure))
  (Default|CallSetSelectedSquare self))

(event Custom|ChangeEnemyOccupied
  (params (IsOccupied :type Boolean))
  (Variables|Default|SetEnemyOccupied IsOccupied)
  (if (Variables|Default|GetEnemyOccupied)
    (Rendering|Material|SetMaterial (Variables|Default|GetStaticMesh) 0 0)
    (else
      (Rendering|Material|SetMaterial (Variables|Default|GetStaticMesh) 0 0))))

(event EventBeginPlay
  (EventDispatchers|BindEventtoSetEnemyOccupied (delegate Custom|ChangeEnemyOccupied))
  (if (Variables|Default|GetEnemyOccupied)
    (Rendering|Material|SetMaterial (Variables|Default|GetStaticMesh) 0 0)
    (else
      (Rendering|Material|SetMaterial (Variables|Default|GetStaticMesh) 0 0))))

(event MouseInput|EventActorBeginCursorOver
  (bind _asmaterial (Utilities|Casting|CastToMaterial (Utilities|Array|Get(acopy) (Rendering|Material|GetMaterials (Variables|Default|GetStaticMesh)))))
  (Variables|Default|SetMaterialCache _asmaterial)
  (if (Variables|Default|GetEnemyOccupied)
    (Rendering|Material|SetMaterial (Variables|Default|GetStaticMesh) 0 0)
    (else
      (Rendering|Material|SetMaterial (Variables|Default|GetStaticMesh) 0 0))))

(event MouseInput|EventActorEndCursorOver
  (Rendering|Material|SetMaterial (Variables|Default|GetStaticMesh) 0 (Variables|Default|GetMaterialCache)))

(fn ConstructionScript)

(fn SetVisibility
  (params (Visible :type Boolean))
  (Rendering|SetVisibility (Variables|Default|GetStaticMesh) Visible false))

(fn SetMoveable
  (params (movable :type Boolean))
  (bind _output_get (Variables|Default|Setmoveable movable))
  (if (Variables|Default|GetEnemyOccupied)
    (if _output_get
      (Rendering|Material|SetMaterial (Variables|Default|GetStaticMesh) 0 0)
      (else
        (Rendering|Material|SetMaterial (Variables|Default|GetStaticMesh) 0 0)))
    (elif _output_get
      (Rendering|Material|SetMaterial (Variables|Default|GetStaticMesh) 0 0)
      (else
        (Rendering|Material|SetMaterial (Variables|Default|GetStaticMesh) 0 0)))))